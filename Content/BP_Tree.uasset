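; BP_Tree is a tree actor that picks a random tree type for itself and reports it at play start.
; The Construction Script casts a random integer, bounded by the ETreeType entry count, to the enum and stores it in Type, so the value re-rolls whenever construction reruns.
; BeginPlay formats the type's name into a message and prints it; overlap and Tick events are unused.
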(event `self.ReceiveBeginPlay`
  (`KismetSystemLibrary.PrintText` (`|FormatText` "\"My Tree Type is {0}\"" (`KismetTextLibrary.Conv_NameToText` (`|GetEnumeratorName` (`self.Type`))))))

(fn `UserConstructionScript`
  (set `self.Type` (cast `ETreeType` (`KismetMathLibrary.Conv_IntToByte` (`KismetMathLibrary.RandomInteger` (enumcount `ETreeType`))))))